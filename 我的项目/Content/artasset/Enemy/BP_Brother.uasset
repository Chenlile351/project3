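; BP_Brother is a character-dialogue Blueprint that shows the Brother's lines one at a time in a WB_Dialogue widget.
; Each Talk event advances an index into the Dialogue array, creating the widget only if none is valid, and sets its text.
; At index 3 it hides the ImageBg image and shows ImageB.
; Once the lines run out it removes the widget, with no index reset.
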(event `/Game/ThirdPerson/Blueprints/BPI_Dialogue.Talk`
  (`/Engine/EditorBlueprintResources/StandardMacros.IncrementInt` (`self.Talkindex`)
    (:`  `
      (if (< (`self.Talkindex`) (`KismetArrayLibrary.Array_Length` (`self.Dialogue`)))
        (`self.UI`
          (:`then`
            _)
          (:`else`
            (bind _returnvalue (`|CreateWidget` "/Game/artasset/music/UI/WB_Dialogue.WB_Dialogue_C" (`GameplayStatics.GetPlayerController` 0)))
            (bind _output_get (set `self.UI` _returnvalue))
            (`UserWidget.AddToViewport` _output_get 0)))
        (`TextBlock.SetText` (`/Game/artasset/music/UI/WB_Dialogue.TalkText` (`self.UI`)) (`KismetTextLibrary.Conv_StringToText` (`|GetArrayItem` (`self.Dialogue`) (`self.Talkindex`))))
        (if (== (`self.Talkindex`) 3)
          (`Widget.SetVisibility` (`/Game/artasset/music/UI/WB_Dialogue.Image_bg` (`self.UI`)) "Hidden")
          (`Widget.SetVisibility` (`/Game/artasset/music/UI/WB_Dialogue.Image_B` (`self.UI`)) "Visible"))
        (else
          (`Widget.RemoveFromParent` (`self.UI`)))))))

(fn `UserConstructionScript`)