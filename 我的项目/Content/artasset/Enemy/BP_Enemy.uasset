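; Enemy pawn that wanders, moves toward the player when it sees them, and opens Project_3_level1 when its Attack component overlaps the player character.
; PawnSensing briefly sets IsSeeingPlayer to start an AI move to the player, then clears it in the same Sequence.
; With that flag clear, Tick feeds a random Delay into Patrol, which moves to a random reachable nearby point.
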(event `self.Attack.OnComponentBeginOverlap`
  (params (OverlappedComponent :type "PrimitiveComponent Object Reference") (OtherActor :type "Actor Object Reference") (OtherComp :type "PrimitiveComponent Object Reference") (OtherBodyIndex :type Integer) (bFromSweep :type Boolean) (SweepResult :type "HitResult Structure (by ref)"))
  (cast `/Game/ThirdPerson/Blueprints/BP_ThirdPersonCharacter` OtherActor)
  (`GameplayStatics.OpenLevel` "Project_3_level1"))

(event `self.PawnSensing.OnSeePawn`
  (params (Pawn :type "Pawn Object Reference"))
  (cast `/Game/ThirdPerson/Blueprints/BP_ThirdPersonCharacter` Pawn)
  (`|ExecutionSequence`
    (:`then_0`
      (set `self.isSeeingPlayer?` true)
      (`self.FollowPlayer`))
    (:`then_1`
      (set `self.isSeeingPlayer?` false))))

(event `FollowPlayer`
  (if (`self.isSeeingPlayer?`)
    (`|AIMoveTo` self (0.0 0.0 0.0) (`GameplayStatics.GetPlayerCharacter` 0))))

(event `Patrol`
  (`|AIMoveTo` self (`NavigationSystemV1.K2_GetRandomReachablePointInRadius` (`self.K2_GetActorLocation`) 500.0 null null) null))

(event `self.ReceiveTick`
  (params (DeltaSeconds :type "Float (single-precision)"))
  (if (not (`self.isSeeingPlayer?`))
    (`KismetSystemLibrary.Delay` (`KismetMathLibrary.RandomFloatInRange` 2.0 5.0))
    (`self.Patrol`)))

(fn `UserConstructionScript`)